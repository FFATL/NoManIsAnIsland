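; BP_BattleMode is the game mode for the battle minigame level, marking the minigame as unlocked in the dialogue system when play begins.
; It initializes the player's HUD, then branches on the level options string to configure the HUD's Darkest widget.
; The main option hides the skip button and turns on random truth giving, while the plot option binds battle victory to open the Chapter Three after-battle level.
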(event Custom|BattleVictory_Event_0
  (Game|OpenLevel(byObjectReference) "/Game/Chapter/Chapter_3_After_Battle/Map/Chapter_Three_After_Battle.Chapter_Three_After_Battle"))

(event EventBeginPlay
  (bind _returnvalue (Game|GetPlayerState 0))
  (bind _returnvalue_2 (Game|GetPlayerController _returnvalue))
  (Class|DialogueSubsystem|SetCheckMapValue (Subsystems|GetDialogueSubsystem) "minigame_unlocked" true)
  (|CallParentFunction _returnvalue_2)
  (bind _asbp_battle_hud (Utilities|Casting|CastToBP_BattleHUD (HUD|GetHUD _returnvalue_2)))
  (switch string (Variables|Default|GetOptionsString)
    (:?main
      (Default|HideSkipGame (Variables|/Game/Battle/Blueprints/BP_BattleHUD.BP_BattleHUD_C|GetDarkestWidgetReference _asbp_battle_hud))
      (Variables|/Game/Battle/Blueprints/BP_Darkest.BP_Darkest_C|SetbRandomTruthGiver (Variables|/Game/Battle/Blueprints/BP_BattleHUD.BP_BattleHUD_C|GetDarkestWidgetReference _asbp_battle_hud) true))
    (:?plot
      (EventDispatchers|AssignBattleVictory (Variables|/Game/Battle/Blueprints/BP_BattleHUD.BP_BattleHUD_C|GetDarkestWidgetReference _asbp_battle_hud) (delegate Custom|BattleVictory_Event_0)))))

(fn ConstructionScript)