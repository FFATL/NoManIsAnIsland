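; BP_SpriteActor is a reusable actor that displays a Paper2D sprite and reports clicks on it.
; SetSpriteAndScale assigns a sprite and scales it in X and Z with Y fixed at 1, while UpdateSprite swaps only the sprite.
; Both functions return the actor itself, and clicking the sprite component calls OnClickedPaperSprite, apparently an event dispatcher for outside listeners.
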(event OnClicked(PaperSprite)
  (params (TouchedComponent :type Primitive%20Component%20Object%20Reference) (ButtonPressed :type Key%20Structure))
  (Default|CallOnClickedPaperSprite))

(event EventBeginPlay)

(event Collision|EventActorBeginOverlap
  (params (OtherActor :type Actor%20Object%20Reference)))

(event EventTick
  (params (DeltaSeconds :type Float%20%28single-precision%29)))

(fn ConstructionScript)

(fn SetSpriteandScale
  (params (Sprite :type Paper%20Sprite%20Object%20Reference) (Width_X :type Float%20%28double-precision%29) (Height_Z :type Float%20%28double-precision%29))
  (bind _papersprite (Variables|Default|GetPaperSprite))
  (Transformation|SetRelativeScale3D _papersprite (Math|Vector|MakeVector Width_X 1.0 Height_Z))
  (Rendering|Components|Sprite|SetSprite _papersprite Sprite)
  (return self))

(fn UpdateSprite
  (params (Sprite :type Paper%20Sprite%20Object%20Reference))
  (Rendering|Components|Sprite|SetSprite (Variables|Default|GetPaperSprite) Sprite)
  (return self))