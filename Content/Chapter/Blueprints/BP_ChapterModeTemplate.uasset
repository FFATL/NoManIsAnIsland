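; BP_ChapterModeTemplate is a chapter mode template Blueprint that provides helper functions for sprite spawning and dialogue state.
; SpawnSpriteActor spawns a BP_SpriteActor at a transform's location and rotation with unit scale, then passes the transform's X and Z scale as sprite width and height.
; SetDialogueCheckMapValue writes a check map value through the DialogueSubsystem, reads it back and prints both results for debugging.
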(fn ConstructionScript)

(fn SpawnSpriteActor
  (params (Transform :type Transform) (Sprite :type Paper%20Sprite%20Object%20Reference))
  (bind (_location _rotation _scale) (Math|Transform|BreakTransform Transform))
  (bind (_x _y _z) (Math|Vector|BreakVector _scale))
  (bind _returnvalue (Game|SpawnActorfromClass "/Game/SpriteActor/BP_SpriteActor.BP_SpriteActor_C" (Math|Transform|MakeTransform _location _rotation) "Undefined" 0 0))
  (bind _selfref (Default|SetSpriteandScale _returnvalue Sprite _x _z))
  (return _selfref))

(fn SetDialogueCheckMapValue
  (params (ConfigKey :type Name) (NewValue :type Boolean))
  (bind _returnvalue (Subsystems|GetDialogueSubsystem))
  (bind _returnvalue_2 (Class|DialogueSubsystem|SetCheckMapValue _returnvalue ConfigKey NewValue))
  (bind _returnvalue_3 (Class|DialogueSubsystem|GetCheckMapValue _returnvalue ConfigKey))
  (Development|PrintText (Utilities|Text|FormatText "Set {key} {value}: {result} [{get_result}]" ConfigKey NewValue _returnvalue_2 _returnvalue_3)))