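; Game mode for the Chapter 3 after-battle scene, which plays a dialogue session and then moves on to Chapter Four.
; On BeginPlay it initializes the first player's HUD, casts it to BP_ChapterHUD and spawns a bridge sprite as scenery.
; The HUD generates a dialogue whose session is set to the after-battle script, with its end delegate bound to open the next level.
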(event Custom|OnDEnd
  (Game|OpenLevel(byObjectReference) "/Game/Chapter/Chapter_4/Map/Chapter_Four.Chapter_Four"))

(event EventBeginPlay
  (bind _returnvalue (Game|GetPlayerController 0))
  (|CallParentFunction _returnvalue)
  (bind _asbp_chapter_hud (Utilities|Casting|CastToBP_ChapterHUD (HUD|GetHUD _returnvalue)))
  (CallFunction|SpawnSpriteActor (Math|Transform|MakeTransform "930.000000,0.000000,77.000000" "0,90.000000, 0" "0.100000,1.000000,0.100000") "/Game/SpriteActor/Bridge_Sprite.Bridge_Sprite")
  (bind _dialoguesessionptr (Default|GenerateNewDialogue _asbp_chapter_hud))
  (EventDispatchers|AssignOnDialogueSessionEnd _dialoguesessionptr (delegate Custom|OnDEnd))
  (Class|DialogueUI|SetSession _dialoguesessionptr "chapter_three_after_battle"))

(fn ConstructionScript)