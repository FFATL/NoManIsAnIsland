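; BP_EndingMode is the ending chapter's game mode, presenting one of three endings and then returning to the main menu.
; On BeginPlay it initializes the chapter HUD, spawns a sprite actor and requests a new dialogue from the HUD.
; The level's options string (?A, ?B or ?C) selects the branch that updates the sprite and sets the dialogue session.
; All three branches bind the session-end event to open the MainMenu level.
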(event Custom|OnReturnMainMenu
  (Game|OpenLevel(byObjectReference) "/Game/MainMenu/Maps/MainMenu.MainMenu"))

(event EventBeginPlay
  (bind _returnvalue (Game|GetPlayerController 0))
  (|CallParentFunction _returnvalue)
  (bind _asbp_chapter_hud (Utilities|Casting|CastToBP_ChapterHUD (HUD|GetHUD _returnvalue)))
  (bind _output_get (Variables|Default|SetLocalHUDRef _asbp_chapter_hud))
  (bind _spriteactorref (CallFunction|SpawnSpriteActor (Math|Transform|MakeTransform "0.000000,0.000000,0.000000" "0,0.000000, 0" "0.200000,1.000000,0.200000")))
  (bind (_dialoguesessionptr _success) (Default|GenerateNewDialogue _output_get))
  (if _success
    (switch string (Variables|Default|GetOptionsString)
      (:?A
        (Default|UpdateSprite _spriteactorref)
        (Class|DialogueUI|SetSession _dialoguesessionptr))
      (:?B
        (Default|UpdateSprite _spriteactorref)
        (Class|DialogueUI|SetSession _dialoguesessionptr))
      (:?C
        (Default|UpdateSprite _spriteactorref)
        (Class|DialogueUI|SetSession _dialoguesessionptr)))
    (EventDispatchers|AssignOnDialogueSessionEnd _dialoguesessionptr (delegate Custom|OnReturnMainMenu))))

(fn ConstructionScript
  (|CallParentFunction))