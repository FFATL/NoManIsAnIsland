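; BP_ChapterThreeMode is the game mode for chapter three, gating progress behind a clickable blocked-bridge sprite.
; On BeginPlay it initializes the HUD, marks the chapter unlocked in the dialogue check map, and spawns the bridge sprite.
; Clicking the bridge unbinds the click and starts the pre-battle dialogue session through the chapter HUD.
; When that session ends, it opens the after-battle level.
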(event Custom|OnBattle
  (Game|OpenLevel(byObjectReference) "/Game/Chapter/Chapter_3_After_Battle/Map/Chapter_Three_After_Battle.Chapter_Three_After_Battle"))

(event Custom|OnBridge
  (EventDispatchers|UnbindEventfromOnClickedPaperSprite (stale EventBeginPlay _spriteactorref) (delegate Custom|OnBridge))
  (bind (_dialoguesessionptr _success) (Default|GenerateNewDialogue (stale EventBeginPlay _output_get)))
  (if _success
    (EventDispatchers|AssignOnDialogueSessionEnd _dialoguesessionptr (delegate Custom|OnBattle))
    (Class|DialogueUI|SetSession _dialoguesessionptr "chapter_three_before_battle")))

(event EventBeginPlay
  (bind _returnvalue (Game|GetPlayerController 0))
  (|CallParentFunction _returnvalue)
  (CallFunction|SetDialogueCheckMapValue "ch3_unlocked" true)
  (bind _asbp_chapter_hud (Utilities|Casting|CastToBP_ChapterHUD (HUD|GetHUD _returnvalue)))
  (bind _output_get (Variables|Default|SetLocalHUDRef _asbp_chapter_hud))
  (bind _spriteactorref (CallFunction|SpawnSpriteActor (Math|Transform|MakeTransform "930.000000,0.000000,77.000000" "0,90.000000, 0" "0.100000,1.000000,0.100000") "/Game/SpriteActor/Bridge_Blocked_Sprite.Bridge_Blocked_Sprite"))
  (EventDispatchers|BindEventtoOnClickedPaperSprite _spriteactorref (delegate Custom|OnBridge)))

(fn ConstructionScript
  (|CallParentFunction))