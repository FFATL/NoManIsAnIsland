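; BP_ChapterOneMode is the chapter one game mode that scripts the chapter's opening story sequence up to the battle.
; It chains dialogue sessions generated by the chapter HUD, using each session-end event to spawn the next clickable Paper sprite.
; Clicking the fight and card sprites starts their dialogues; a signal during the fight dialogue removes the fight sprite.
; When the final dialogue ends, it opens the Chapter_One_After_Battle level.
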(event Custom|OnDEnd_bookworm_fight_pre
  (bind _spriteactorref (CallFunction|SpawnSpriteActor (Math|Transform|MakeTransform "930.000000,180.000000,77.000000" "0,90.000000, 0" "0.100000,1.000000,0.100000") "/Game/SpriteActor/Fight_Sprite.Fight_Sprite"))
  (EventDispatchers|BindEventtoOnClickedPaperSprite _spriteactorref (delegate Custom|OnDEnd_bookworm_fight_dialogue)))

(event Custom|OnDEnd_bookworm_before_battle_pre
  (bind _spriteactorref (CallFunction|SpawnSpriteActor (Math|Transform|MakeTransform "1320.000000,0.000000,66.000000" "0,90.000000, 0" "0.100000,1.000000,0.100000") "/Game/Character/Card_Sprite.Card_Sprite"))
  (EventDispatchers|BindEventtoOnClickedPaperSprite _spriteactorref (delegate Custom|OnDEnd_bookworm_before_battle_dialogue)))

(event Custom|OnDEnd_bookworm_before_battle_dialogue
  (Actor|DestroyActor (stale Custom|OnDEnd_bookworm_before_battle_pre _spriteactorref))
  (bind _dialoguesessionptr (Default|GenerateNewDialogue (Variables|Default|GetLocalHUDRef)))
  (Class|DialogueUI|SetSession _dialoguesessionptr "chapter_one_before_battle")
  (EventDispatchers|BindEventtoOnDialogueSessionEnd _dialoguesessionptr (delegate Custom|OnStartBattle)))

(event Custom|OnDestroyFightSprite
  (Actor|DestroyActor (stale Custom|OnDEnd_bookworm_fight_pre _spriteactorref)))

(event Custom|OnDEnd_bookworm_fight_dialogue
  (EventDispatchers|UnbindEventfromOnClickedPaperSprite (stale Custom|OnDEnd_bookworm_fight_pre _spriteactorref) (delegate Custom|OnDEnd_bookworm_fight_dialogue))
  (bind _dialoguesessionptr (Default|GenerateNewDialogue (Variables|Default|GetLocalHUDRef)))
  (EventDispatchers|BindEventtoOnDialogueSessionEnd _dialoguesessionptr (delegate Custom|OnDEnd_bookworm_before_battle_pre))
  (EventDispatchers|BindEventtoOnDialogueSignalOne _dialoguesessionptr (delegate Custom|OnDestroyFightSprite))
  (Class|DialogueUI|SetSession _dialoguesessionptr "chapter_one_bookworm_fight"))

(event Custom|OnStartBattle
  (Game|OpenLevel(byObjectReference) "/Game/Chapter/Chapter_1_After_Battle/Map/Chapter_One_After_Battle.Chapter_One_After_Battle"))

(event EventBeginPlay
  (bind _returnvalue (Game|GetPlayerController 0))
  (|CallParentFunction _returnvalue)
  (bind _asbp_chapter_hud (Utilities|Casting|CastToBP_ChapterHUD (HUD|GetHUD _returnvalue)))
  (bind _output_get (Variables|Default|SetLocalHUDRef _asbp_chapter_hud))
  (bind _dialoguesessionptr (Default|GenerateNewDialogue _output_get))
  (Class|DialogueUI|SetSession _dialoguesessionptr "chapter_one_start")
  (EventDispatchers|AssignOnDialogueSessionEnd _dialoguesessionptr (delegate Custom|OnDEnd_bookworm_fight_pre)))

(fn ConstructionScript)