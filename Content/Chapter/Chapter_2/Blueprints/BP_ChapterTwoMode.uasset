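; Game mode for Chapter 2, a point-and-click puzzle that spawns a clickable door and two key-bearing trees as paper sprites.
; Clicking each starts a HUD dialogue session whose signals swap sprites and set progress flags.
; The trees respond only after the door is checked; finishing both sets a dialogue check value for the door to open.
; The door's dialogue then signals the opening and loads Chapter 3 when it ends.
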(event EventBeginPlay
  (bind _returnvalue (Game|GetPlayerController 0))
  (|CallParentFunction _returnvalue)
  (CallFunction|SetDialogueCheckMapValue "ch2_unlocked" true)
  (bind _asbp_chapter_hud (Utilities|Casting|CastToBP_ChapterHUD (HUD|GetHUD _returnvalue)))
  (Variables|Default|SetLocalHUDRef _asbp_chapter_hud)
  (bind _spriteactorref (CallFunction|SpawnSpriteActor (Math|Transform|MakeTransform "2469.000000,0.000000,133.000000" "0,90.000000, 0" "0.300000,1.000000,0.300000") "/Game/SpriteActor/Door_Sprite.Door_Sprite"))
  (EventDispatchers|BindEventtoOnClickedPaperSprite _spriteactorref (delegate CGDoor))
  (bind _spriteactorref_2 (CallFunction|SpawnSpriteActor (Math|Transform|MakeTransform "2015.000000,576.000000,163.000000" "0,90.000000, 0" "0.300000,1.000000,0.300000") "/Game/SpriteActor/Tree_Nest_Key_Sprite.Tree_Nest_Key_Sprite"))
  (EventDispatchers|BindEventtoOnClickedPaperSprite _spriteactorref_2 (delegate CGCard))
  (bind _spriteactorref_3 (CallFunction|SpawnSpriteActor (Math|Transform|MakeTransform "2015.000000,-518.000000,163.000000" "0,90.000000, 0" "0.300000,1.000000,0.300000") "/Game/SpriteActor/Tree_Chrysalis_Key_Sprite.Tree_Chrysalis_Key_Sprite"))
  (EventDispatchers|BindEventtoOnClickedPaperSprite _spriteactorref_3 (delegate CGBookworm)))

(fn ConstructionScript
  (|CallParentFunction))

(event Custom|OnDoor
  (bind (_dialoguesessionptr _success) (Default|GenerateNewDialogue (Variables|Default|GetLocalHUDRef)))
  (if _success
    (EventDispatchers|BindEventtoOnDialogueSignalOne _dialoguesessionptr (delegate Custom|OnSetDoorChecked))
    (EventDispatchers|BindEventtoOnDialogueSignalTwo _dialoguesessionptr (delegate Custom|OnSetDoorOpen))
    (EventDispatchers|BindEventtoOnDialogueSessionEnd _dialoguesessionptr (delegate Custom|OnNextChapter))
    (Class|DialogueUI|SetSession _dialoguesessionptr "chapter_two_locked_door")))

(event Custom|OnSetDoorOpen
  (Variables|Default|SetbDoorCheckedAndOpen true)
  (Default|UpdateSprite (|Inputs) "/Game/SpriteActor/Door_Open_Sprite.Door_Open_Sprite"))

(event Custom|OnSetDoorChecked
  (Variables|Default|SetbDoorChecked true))

(event Custom|OnNextChapter
  (if (Variables|Default|GetbDoorCheckedAndOpen)
    (Game|OpenLevel(byObjectReference) "/Game/Chapter/Chapter_3/Map/Chapter_Three.Chapter_Three")))

(event Custom|OnCard
  (if (Variables|Default|GetbDoorChecked)
    (if (not (Variables|Default|GetbNestKeyGot))
      (bind (_dialoguesessionptr _success) (Default|GenerateNewDialogue (Variables|Default|GetLocalHUDRef)))
      (if _success
        (Class|DialogueUI|SetSession _dialoguesessionptr "chapter_two_nest_card")
        (EventDispatchers|AssignOnDialogueSignalOne _dialoguesessionptr (delegate Custom|OnGetNestKey))
        (EventDispatchers|BindEventtoOnDialogueSessionEnd _dialoguesessionptr (delegate Custom|OnCardEnd))))))

(event Custom|OnGetNestKey
  (Default|UpdateSprite (|Inputs) "/Game/SpriteActor/Tree_Nest_Sprite.Tree_Nest_Sprite"))

(event Custom|OnCardEnd
  (Variables|Default|SetbNestKeyGot true)
  (if (Variables|Default|GetbChryKeyGot)
    (Class|DialogueSubsystem|SetCheckMapValue (Subsystems|GetDialogueSubsystem) "ch2_door_open" true)))

(event Custom|OnGetChryKey
  (Default|UpdateSprite (|Inputs) "/Game/SpriteActor/Tree_Chrysalis_Sprite.Tree_Chrysalis_Sprite"))

(event Custom|OnBookwormEnd
  (Variables|Default|SetbChryKeyGot true)
  (if (Variables|Default|GetbNestKeyGot)
    (Class|DialogueSubsystem|SetCheckMapValue (Subsystems|GetDialogueSubsystem) "ch2_door_open" true)))

(event Custom|OnBookworm
  (if (Variables|Default|GetbDoorChecked)
    (if (not (Variables|Default|GetbChryKeyGot))
      (bind (_dialoguesessionptr _success) (Default|GenerateNewDialogue (Variables|Default|GetLocalHUDRef)))
      (if _success
        (Class|DialogueUI|SetSession _dialoguesessionptr "chapter_two_chrysalis_bookworm")
        (EventDispatchers|AssignOnDialogueSignalOne _dialoguesessionptr (delegate Custom|OnGetChryKey))
        (EventDispatchers|BindEventtoOnDialogueSessionEnd _dialoguesessionptr (delegate Custom|OnBookwormEnd))))))