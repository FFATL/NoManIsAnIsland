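; Chapter four game mode that runs the uphill-mount dialogue session and routes the story to one of three endings.
; BeginPlay shows a forest bridge sprite and starts the session through the chapter HUD.
; Two generic dialogue signals act as a state machine: handlers rebind them at each branch and swap scene and ending sprites.
; Session end opens the Chapter_Ending level with option A, B or C.
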(event Custom|OnGoEndingA
  (Game|OpenLevel(byObjectReference) "/Game/Chapter/Ending/Map/Chapter_Ending.Chapter_Ending" true "A"))

(event Custom|OnReachTop
  (Actor|DestroyActor (stale EventBeginPlay _spriteactorref))
  (EventDispatchers|UnbindEventfromOnDialogueSignalOne (stale EventBeginPlay _dialoguesessionptr) (delegate Custom|OnReachTop))
  (EventDispatchers|BindEventtoOnDialogueSignalOne (stale EventBeginPlay _dialoguesessionptr) (delegate Custom|OnEndingA))
  (EventDispatchers|BindEventtoOnDialogueSignalTwo (stale EventBeginPlay _dialoguesessionptr) (delegate Custom|OnBranchA)))

(event Custom|OnGoEndingC
  (Game|OpenLevel(byObjectReference) "/Game/Chapter/Ending/Map/Chapter_Ending.Chapter_Ending" true "C"))

(event Custom|OnEndingA
  (Development|PrintString "The sky is the limit.")
  (EventDispatchers|UnbindEventfromOnDialogueSignalTwo (stale EventBeginPlay _dialoguesessionptr) (delegate Custom|OnBranchA))
  (EventDispatchers|BindEventtoOnDialogueSignalTwo (stale EventBeginPlay _dialoguesessionptr) (delegate Custom|OnPlayEndACG))
  (EventDispatchers|BindEventtoOnDialogueSessionEnd (stale EventBeginPlay _dialoguesessionptr) (delegate Custom|OnGoEndingA)))

(event Custom|OnBranchA
  (EventDispatchers|UnbindEventfromOnDialogueSignalOne (stale EventBeginPlay _dialoguesessionptr) (delegate Custom|OnEndingA))
  (EventDispatchers|BindEventtoOnDialogueSignalOne (stale EventBeginPlay _dialoguesessionptr) (delegate Custom|OnEndingB))
  (EventDispatchers|UnbindEventfromOnDialogueSignalTwo (stale EventBeginPlay _dialoguesessionptr) (delegate Custom|OnBranchA))
  (EventDispatchers|BindEventtoOnDialogueSignalTwo (stale EventBeginPlay _dialoguesessionptr) (delegate Custom|OnEndingC))
  (bind _spriteactorref (CallFunction|SpawnSpriteActor (Math|Transform|MakeTransform "306.000000,0.000000,311.000000" "0,90.000000, 0" "0.200000,1.000000,0.200000") "/Game/SpriteActor/CG/Rolling_Sprite.Rolling_Sprite")))

(event Custom|OnEndingB
  (Development|PrintString "Down to earth.")
  (Actor|DestroyActor (stale Custom|OnBranchA _spriteactorref))
  (CallFunction|SpawnSpriteActor (Math|Transform|MakeTransform "-355.000000,0.000000,316.000000" "0,90.000000, 0" "0.300000,1.000000,0.300000") "/Game/SpriteActor/CG/EndingB_Sprite.EndingB_Sprite")
  (EventDispatchers|BindEventtoOnDialogueSessionEnd (stale EventBeginPlay _dialoguesessionptr) (delegate Custom|OnGoEndingB)))

(event Custom|OnEndingC
  (Development|PrintString "No man is an island.")
  (EventDispatchers|UnbindEventfromOnDialogueSignalOne (stale EventBeginPlay _dialoguesessionptr) (delegate Custom|OnEndingB))
  (EventDispatchers|BindEventtoOnDialogueSignalOne (stale EventBeginPlay _dialoguesessionptr) (delegate Custom|OnLeaveTree))
  (EventDispatchers|BindEventtoOnDialogueSessionEnd (stale EventBeginPlay _dialoguesessionptr) (delegate Custom|OnGoEndingC)))

(event Custom|OnLeaveTree
  (Actor|DestroyActor (stale Custom|OnBranchA _spriteactorref)))

(event Custom|OnPlayEndACG
  (CallFunction|SpawnSpriteActor (Math|Transform|MakeTransform "-336.000000,0.000000,412.000000" "0,90.000000, 0" "0.300000,1.000000,0.300000") "/Game/SpriteActor/CG/EndingA_Sprite.EndingA_Sprite"))

(event Custom|OnGoEndingB
  (Game|OpenLevel(byObjectReference) "/Game/Chapter/Ending/Map/Chapter_Ending.Chapter_Ending" true "B"))

(event EventBeginPlay
  (bind _returnvalue (Game|GetPlayerController 0))
  (|CallParentFunction _returnvalue)
  (bind _asbp_chapter_hud (Utilities|Casting|CastToBP_ChapterHUD (HUD|GetHUD _returnvalue)))
  (bind _output_get (Variables|Default|SetLocalHUDRef _asbp_chapter_hud))
  (bind _spriteactorref (CallFunction|SpawnSpriteActor (Math|Transform|MakeTransform "19.000000,-30.000000,335.000000" "0,90.000000, 0") "/Game/Chapter/Chapter_4/Map/forest-bridge_CHJ9QS9YWP_Sprite.forest-bridge_CHJ9QS9YWP_Sprite"))
  (bind (_dialoguesessionptr _success) (Default|GenerateNewDialogue _output_get))
  (if _success
    (EventDispatchers|BindEventtoOnDialogueSignalOne _dialoguesessionptr (delegate Custom|OnReachTop))
    (Class|DialogueUI|SetSession _dialoguesessionptr "chapter_four_mount_uphill")
    (Class|DialogueUI|SetNeedNextSceneHint _dialoguesessionptr true)))

(fn ConstructionScript
  (|CallParentFunction))